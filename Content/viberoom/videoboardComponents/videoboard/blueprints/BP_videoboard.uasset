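; Video board actor that slides open and closed and plays a video through a Media Player.
; SelectVB toggles the board: timelines lerp the border between its start position and a lower one, with base, screen and widget shown after opening and hidden as closing begins, along with their collision.
; Toggle opens the media source on first use while the board is open, then switches play and pause; closing via SelectVB pauses playback.
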(event Custom|startvideo
  (bind _returnvalue (Media|MediaPlayer|OpenSource (Variables|Default|Getmediaplayer) (Variables|Default|Getvideo%20source)))
  (Variables|Default|SethasStarted? _returnvalue))

(event Custom|playvideo
  (bind _mediaplayer (Variables|Default|Getmediaplayer))
  (if (Class|MediaPlayer|IsPaused _mediaplayer)
    (Media|MediaPlayer|Play _mediaplayer :!class /Script/MediaAssets.MediaPlayer)))

(event Custom|pausevideo
  (bind _mediaplayer (Variables|Default|Getmediaplayer))
  (if (not (Class|MediaPlayer|IsPaused _mediaplayer))
    (Sequencer|Player|Pause _mediaplayer)))

(event Custom|close_video_board
  (bind _widget (Variables|Default|GetWidget))
  (if (Variables|Default|Getisopen?)
    (Collision|SetCollisionEnabled _widget "NoCollision")
    (Development|SetHiddeninGame _widget true false)
    (CallFunction|DisableComponent (Variables|Default|Getvideoboard_VBBase))
    (CallFunction|DisableComponent (Variables|Default|Getvideoboard_VBScreen))
    (bind _newtrack_0 (Timeline|borderanimationtimeline2 PlayFromStart)
      (:Update
        (Transformation|SetWorldLocation (Variables|Default|Getvideoboard_VBBBorder) (Math|Vector|Lerp(Vector) (Variables|Default|GetVBBfinalLocation) (Variables|Default|GetVBBinitialLocation) _newtrack_0) false false))
      (:Finished
        (Variables|Default|Setisopen? false)))))

(event Custom|open_video_board
  (bind _widget (Variables|Default|GetWidget))
  (if (not (Variables|Default|Getisopen?))
    (bind _track0 (Timeline|borderanimationtimeline PlayFromStart)
      (:Update
        (Transformation|SetWorldLocation (Variables|Default|Getvideoboard_VBBBorder) (Math|Vector|Lerp(Vector) (Variables|Default|GetVBBinitialLocation) (Variables|Default|GetVBBfinalLocation) _track0) false false))
      (:Finished
        (CallFunction|EnableComponent (Variables|Default|Getvideoboard_VBBase))
        (CallFunction|EnableComponent (Variables|Default|Getvideoboard_VBScreen))
        (Development|SetHiddeninGame _widget false false)
        (Collision|SetCollisionEnabled _widget "QueryAndPhysics")
        (Variables|Default|Setisopen? true)))))

(event EventBeginPlay
  (bind _videoboard_vbbborder (Variables|Default|Getvideoboard_VBBBorder))
  (bind _widget (Variables|Default|GetWidget))
  (bind _returnvalue (Transformation|GetWorldLocation _videoboard_vbbborder))
  (CallFunction|DisableComponent (Variables|Default|Getvideoboard_VBBase))
  (CallFunction|DisableComponent (Variables|Default|Getvideoboard_VBScreen))
  (Development|SetHiddeninGame _widget true false)
  (Collision|SetCollisionEnabled _widget "NoCollision")
  (Variables|Default|SetVBBinitialLocation _returnvalue)
  (Variables|Default|SetVBBfinalLocation (- _returnvalue "0, 0,330.000000")))

(event EventSelectVB
  (if (Variables|Default|Getisopen?)
    (if (Audio|Components|Audio|IsPlaying (Variables|Default|Getmediaplayer))
      (CallFunction|Pausevideo))
    (CallFunction|CloseVideoBoard)
    (else
      (CallFunction|OpenVideoBoard))))

(event EventToggle
  (if (Variables|Default|GethasStarted?)
    (if (Audio|Components|Audio|IsPlaying (Variables|Default|Getmediaplayer))
      (CallFunction|Pausevideo)
      (else
        (CallFunction|Playvideo)))
    (elif (Variables|Default|Getisopen?)
      (CallFunction|Startvideo))))

(fn ConstructionScript)

(fn DisableComponent
  (params (NewParam :type Static%20Mesh%20Component%20Object%20Reference))
  (Development|SetHiddeninGame NewParam true false)
  (Collision|SetCollisionEnabled NewParam "NoCollision")
  (Components|Tick|SetComponentTickEnabled NewParam false)
  (return))

(fn EnableComponent
  (params (NewParam :type Static%20Mesh%20Component%20Object%20Reference))
  (Development|SetHiddeninGame NewParam false false)
  (Collision|SetCollisionEnabled NewParam "QueryAndPhysics")
  (Components|Tick|SetComponentTickEnabled NewParam true)
  (return))