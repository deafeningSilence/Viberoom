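; Studious assistant character that listens to scripted requests and presents a book.
; Selection gives a held book or, when not listening, starts listening and shows the next of three request widgets via Reqnum, setting HeardText for later ones.
; BkEnterHit ends listening and hides widgets; FindBook expands the bookshelf, then the book.
; Timelines animate dish, shelf and book, while face materials signal listening, searching and pause state.
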(event Custom|Stop%20Listening
  (Rendering|Material|SetMaterial (Variables|Default|GetSkeletalMesh) 0 (Variables|Default|Getcurrent%20material))
  (Variables|Default|Setlistening? false)
  (bind _newtrack_0 (Timeline|dish%20minimizing%20timeline PlayFromStart)
    (:Update
      (Transformation|SetRelativeScale3D (Variables|Default|GetBP_dish) (Math|Vector|Lerp(Vector) (Variables|Default|Getdish%20final%20scale) (Variables|Default|Getdish%20initial%20scale) _newtrack_0)))))

(event Custom|Find%20Book
  (Variables|Default|Setholdingbook? true)
  (Rendering|Material|SetMaterial (Variables|Default|GetSkeletalMesh) 0 "/Game/viberoom/studious/materials/M_studious_Ueyes.M_studious_Ueyes")
  (bind _newtrack_0 (Timeline|bookshelf%20expanding%20timeline PlayFromStart)
    (:Update
      (Transformation|SetRelativeScale3D (Variables|Default|Getbookshelf) (Math|Vector|Lerp(Vector) (Variables|Default|Getbookshelf%20initial%20scale) (Variables|Default|Getbookshelf%20final%20scale) _newtrack_0)))
    (:Finished
      (bind _newtrack_0_2 (Timeline|book%20expanding%20timeline PlayFromStart)
        (:Update
          (Transformation|SetRelativeScale3D (Variables|Default|GetBP_studiousbook) (Math|Vector|Lerp(Vector) (Variables|Default|GetBook%20initial%20scale) (Variables|Default|GetBook%20final%20scale) _newtrack_0_2)))))))

(event Custom|Give%20book
  (Variables|Default|Setholdingbook? false)
  (Rendering|Material|SetMaterial (Variables|Default|GetSkeletalMesh) 0 (Variables|Default|Getcurrent%20material))
  (Transformation|SetRelativeScale3D (Variables|Default|GetBP_studiousbook) (Variables|Default|GetBook%20initial%20scale))
  (bind _newtrack_0 (Timeline|bookshelf%20minimizing%20timeline PlayFromStart)
    (:Update
      (Transformation|SetRelativeScale3D (Variables|Default|Getbookshelf) (Math|Vector|Lerp(Vector) (Variables|Default|Getbookshelf%20final%20scale) (Variables|Default|Getbookshelf%20initial%20scale) _newtrack_0)))))

(event Custom|Start%20Listening
  (Rendering|Material|SetMaterial (Variables|Default|GetSkeletalMesh) 0 "/Game/viberoom/studious/materials/M_studious_listening.M_studious_listening")
  (Utilities|FlowControl|Delay 0.1)
  (Variables|Default|Setlistening? true)
  (bind _newtrack_0 (Timeline|dish%20expanding%20timeline PlayFromStart)
    (:Update
      (Transformation|SetRelativeScale3D (Variables|Default|GetBP_dish) (Math|Vector|Lerp(Vector) (Variables|Default|Getdish%20initial%20scale) (Variables|Default|Getdish%20final%20scale) _newtrack_0)))
    (:Finished
      (bind _newtrack_1 (Timeline|dish%20rotating%20timeline PlayFromStart)
        (:Update
          (Transformation|SetRelativeRotation (Variables|Default|GetBP_dish) (Math|Rotator|Lerp(Rotator) (Variables|Default|GetDish%20initial%20rotation) (Variables|Default|GetDish%20final%20rotation) _newtrack_1) false false))))))

(event Collision|EventActorBeginOverlap
  (params (OtherActor :type Actor%20Object%20Reference)))

(event EventBkEnterHit
  (bind _widget1 (Variables|Default|GetWidget1))
  (CallFunction|StopListening)
  (Development|SetHiddeninGame _widget1 true false)
  (Collision|SetCollisionEnabled _widget1 "NoCollision")
  (Components|Tick|SetComponentTickEnabled _widget1 false))

(event EventStudiousSelected
  (bind _widget2 (Variables|Default|GetWidget2))
  (bind _widget3 (Variables|Default|Getwidget3))
  (bind _widget1 (Variables|Default|GetWidget1))
  (if (not (Variables|Default|Getlistening?))
    (if (Variables|Default|Getholdingbook?)
      (CallFunction|GiveBook)
      (else
        (switch int (Variables|Default|Getreqnum)
          (:0
            (CallFunction|StartListening)
            (Development|SetHiddeninGame _widget1 false false)
            (Collision|SetCollisionEnabled _widget1 "QueryAndPhysics")
            (Components|Tick|SetComponentTickEnabled _widget1 true)
            (Variables|Default|Setreqnum (+ (Variables|Default|Getreqnum) 1)))
          (:1
            (CallFunction|StartListening)
            (Development|SetHiddeninGame _widget2 false false)
            (Collision|SetCollisionEnabled _widget2 "QueryAndPhysics")
            (Components|Tick|SetComponentTickEnabled _widget2 true)
            (Variables|Default|Setheard%20text "hey studious can you give me a notebook")
            (Variables|Default|Setreqnum (+ (Variables|Default|Getreqnum) 1)))
          (:2
            (CallFunction|StartListening)
            (Development|SetHiddeninGame _widget3 false false)
            (Collision|SetCollisionEnabled _widget3 "QueryAndPhysics")
            (Components|Tick|SetComponentTickEnabled _widget3 true)
            (Variables|Default|Setheard%20text "define virtual reality")))))))

(event EventTick
  (params (DeltaSeconds :type Float%20%28single-precision%29)))

(event EventBeginPlay
  (bind _widget1 (Variables|Default|GetWidget1))
  (Input|EnableInput (Game|GetPlayerController 0))
  (Transformation|SetRelativeScale3D (Variables|Default|Getbookshelf) (Variables|Default|Getbookshelf%20initial%20scale))
  (Transformation|SetRelativeScale3D (Variables|Default|GetBP_studiousbook) (Variables|Default|Getbook%20initial%20scale))
  (Transformation|SetRelativeScale3D (Variables|Default|GetBP_dish) (Variables|Default|Getdish%20initial%20scale))
  (Variables|Default|Setlistening? false)
  (Variables|Default|Setholdingbook? false)
  (Development|SetHiddeninGame _widget1 true false)
  (Collision|SetCollisionEnabled _widget1 "NoCollision")
  (Components|Tick|SetComponentTickEnabled _widget1 false))

(event Input|ActionEvents|InputActionpause
  (params (Key :type Key%20Structure))
  (:Pressed
    (if (Variables|Default|Getispaused?)
      (bind _output_get (Variables|Default|Setcurrent%20material "/Game/viberoom/studious/materials/M_studious_idle.M_studious_idle"))
      (Rendering|Material|SetMaterial (Variables|Default|GetSkeletalMesh) 0 _output_get)
      (Variables|Default|Setispaused? false)
      (else
        (bind _output_get_2 (Variables|Default|Setcurrent%20material "/Game/viberoom/studious/materials/M_studious_paused.M_studious_paused"))
        (Rendering|Material|SetMaterial (Variables|Default|GetSkeletalMesh) 0 _output_get_2)
        (Variables|Default|Setispaused? true)))))

(fn ConstructionScript)