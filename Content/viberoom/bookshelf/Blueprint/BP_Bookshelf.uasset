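; Bookshelf Blueprint that handles putting a selected book back in its original place when it is deselected.
; The bookDeselcted event hides the AddToTable and Deselect components, then plays a timeline.
; The timeline interpolates BPClosedbook's world location from the shelf's mid location to its initial location, and its rotation from the final to the initial value.
; Selection logic and the setting of those stored transforms are absent from this graph.
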(event Custom|book%20Deselcted
  (Rendering|SetVisibility (Variables|Default|GetaddToTable) false false)
  (bind _newtrack_0 (Timeline|Timeline_1 Play)
    (:Update
      (Transformation|SetWorldLocation (Variables|Default|GetBP_closedbook) (Math|Vector|Lerp(Vector) (Variables|Default|Getbookshelfmidlocation) (Variables|Default|Getinitialbooklocation) _newtrack_0) false false)
      (Transformation|SetWorldRotation (Variables|Default|GetBP_closedbook) (Math|Rotator|Lerp(Rotator) (Variables|Default|Getbookfinalrotation) (Variables|Default|Getinitialbookrotation) _newtrack_0) false false))))

(event Collision|EventActorBeginOverlap
  (params (OtherActor :type Actor%20Object%20Reference)))

(event EventTick
  (params (DeltaSeconds :type Float%20%28single-precision%29)))

(fn ConstructionScript)