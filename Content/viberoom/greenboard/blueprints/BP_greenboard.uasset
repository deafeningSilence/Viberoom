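; Greenboard actor for the viberoom that takes chalk drawing on a render target and can swap its board material.
; BeginPlay creates a chalk material instance and clears the render target; DrawOnGreenboard feeds a 2D location into that material and draws it to the target.
; NumPad 7 advances a counter through two preset board materials, while NumPad 9 restores the greenboard material without resetting the counter or render target.
; The EnableInput call is unconnected.
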(event Custom|Draw%20On%20Greenboard
  (params (Location%20To%20Draw :type Vector%202D%20Structure))
  (bind _chalk_mi (Variables|Default|Getchalk_MI))
  (Rendering|Material|SetVectorParameterValue _chalk_mi "drawLocation" (Math|Conversions|ToLinearColor(Vector) (Math|Conversions|ToVector(Vector2D) Location%20To%20Draw)) :!class /Script/Engine.MaterialInstanceDynamic)
  (Rendering|DrawMaterialtoRenderTarget "/Game/viberoom/greenboard/textures/RT_greenboard.RT_greenboard" _chalk_mi))

(event Custom|ClearBoard
  (Rendering|Material|SetMaterial (Variables|Default|Getboard) 0 "/Game/viberoom/greenboard/materials/M_greenboard.M_greenboard"))

(event EventBeginPlay
  (bind _returnvalue (Rendering|Material|CreateDynamicMaterialInstance "/Game/viberoom/greenboard/materials/M_chalk.M_chalk" :!class /Script/Engine.KismetMaterialLibrary))
  (Variables|Default|Setchalk_MI _returnvalue)
  (Rendering|ClearRenderTarget2D "/Game/viberoom/greenboard/textures/RT_greenboard.RT_greenboard"))

(event Collision|EventActorBeginOverlap
  (params (OtherActor :type Actor%20Object%20Reference)))

(event EventTick
  (params (DeltaSeconds :type Float%20%28single-precision%29)))

(event Input|KeyboardEvents|NumPadSeven
  (params (Key :type Key%20Structure :default "AnyKey"))
  (:Pressed
    (bind _output_get (Variables|Default|Setintcur (+ (Variables|Default|Getintcur) 1)))
    (switch int _output_get
      (:1
        (Rendering|Material|SetMaterial (Variables|Default|Getboard) 0 "/Game/viberoom/greenboard/materials/Mgb2.Mgb2"))
      (:2
        (Rendering|Material|SetMaterial (Variables|Default|Getboard) 0 "/Game/viberoom/greenboard/materials/Mgb3.Mgb3")))))

(event Input|KeyboardEvents|NumPadNine
  (params (Key :type Key%20Structure :default "AnyKey"))
  (:Pressed
    (CallFunction|ClearBoard)))

(fn ConstructionScript)