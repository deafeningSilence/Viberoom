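; Whiteboard actor that slides between three preset world locations (left, middle and right), starting at the left on BeginPlay.
; MoveBoardRight and MoveBoardLeft step it one position by checking CurrentPosition and calling the matching move event.
; Each transition has its own timeline that lerps the root's location between stored vectors.
; CurrentPosition updates only when a timeline finishes, so a repeat call mid-move restarts that slide.
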(event Custom|Move%20To%20Pos%20Mid
  (switch int (Variables|Default|GetcurrentPosition)
    (:0
      (bind _newtrack_1 (Timeline|righttomid PlayFromStart)
        (:Update
          (Transformation|SetWorldLocation (Variables|Default|GetDefaultSceneRoot) (Math|Vector|Lerp(Vector) (Variables|Default|GetrightPosVector) (Variables|Default|GetmidPosVector) _newtrack_1) false false))
        (:Finished
          (Variables|Default|SetcurrentPosition 1))))
    (:2
      (bind _newtrack_1_2 (Timeline|lefttomid PlayFromStart)
        (:Update
          (Transformation|SetWorldLocation (Variables|Default|GetDefaultSceneRoot) (Math|Vector|Lerp(Vector) (Variables|Default|GetleftPosVector) (Variables|Default|GetmidPosVector) _newtrack_1_2) false false))
        (:Finished
          (Variables|Default|SetcurrentPosition 1))))))

(event Custom|move%20to%20pos%20right
  (if (== (Variables|Default|GetcurrentPosition) 1)
    (bind _newtrack_0 (Timeline|midtoright PlayFromStart)
      (:Update
        (Transformation|SetWorldLocation (Variables|Default|GetDefaultSceneRoot) (Math|Vector|Lerp(Vector) (Variables|Default|GetmidPosVector) (Variables|Default|GetrightPosVector) _newtrack_0) false false))
      (:Finished
        (Variables|Default|SetcurrentPosition 0)))))

(event Custom|move%20to%20pos%20left
  (if (== (Variables|Default|GetcurrentPosition) 1)
    (bind _newtrack_1 (Timeline|midtoleft PlayFromStart)
      (:Update
        (Transformation|SetWorldLocation (Variables|Default|GetDefaultSceneRoot) (Math|Vector|Lerp(Vector) (Variables|Default|GetmidPosVector) (Variables|Default|GetleftPosVector) _newtrack_1) false false))
      (:Finished
        (Variables|Default|SetcurrentPosition 2)))))

(event EventBeginPlay
  (Variables|Default|SetcurrentPosition 2)
  (Transformation|SetWorldLocation (Variables|Default|GetDefaultSceneRoot) (Variables|Default|GetleftPosVector) false false))

(event Collision|EventActorBeginOverlap
  (params (OtherActor :type Actor%20Object%20Reference)))

(event EventMoveBoardRight
  (switch int (Variables|Default|GetcurrentPosition)
    (:1
      (CallFunction|MovetoPosRight))
    (:2
      (CallFunction|MovetoPosMid))))

(event EventTick
  (params (DeltaSeconds :type Float%20%28single-precision%29)))

(event EventMoveBoardLeft
  (switch int (Variables|Default|GetcurrentPosition)
    (:0
      (CallFunction|MovetoPosMid))
    (:1
      (CallFunction|MovetoPosLeft))))

(fn ConstructionScript)