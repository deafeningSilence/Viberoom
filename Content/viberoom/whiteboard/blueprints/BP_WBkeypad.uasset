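; BP_WBkeypad is a whiteboard keypad actor that hosts the WB_WBKeypad UMG widget through its Widget component.
; On BeginPlay it casts the hosted widget and hands it the actor's WidgetInteraction reference.
; The Enter-pressed handler is empty, and both its binding and a debug print of the TargetDisplay keypad text are unwired, so neither runs.
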(event Custom|enterPressedEvent_0)

(event EventBeginPlay
  (bind _aswb_wbkeypad (Utilities|Casting|CastToWB_WBKeypad (UserInterface|GetUserWidgetObject (Variables|Default|GetWidget))))
  (Variables|/Game/viberoom/whiteboard/blueprints/WB_WBkeypad.WB_WBKeypad_C|SetwidgetInteraction _aswb_wbkeypad (Variables|Default|GetWidgetInteraction)))

(event Collision|EventActorBeginOverlap
  (params (OtherActor :type Actor%20Object%20Reference)))

(event EventTick
  (params (DeltaSeconds :type Float%20%28single-precision%29)))

(fn ConstructionScript)