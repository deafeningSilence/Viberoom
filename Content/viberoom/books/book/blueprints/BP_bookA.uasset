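; BP_bookA is a book actor that the player opens and pages through with the gamepad D-pad.
; Right or Up opens the closed book or flips right and increments the page number; Left or Down flips left.
; Flips pulse boolean flags, while timed delays swap cover and page visibility on opening and right flips between two spreads.
; Left flips leave visibility unchanged, and the close event is never triggered here.
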(event Custom|open%20book
  (Variables|Default|SetisClosed? false)
  (Rendering|SetVisibility (Variables|Default|Getcover) false false)
  (Utilities|FlowControl|Delay 0.8)
  (Rendering|SetVisibility (Variables|Default|Getleftpage1) true false))

(event Custom|flip%20right
  (Rendering|SetVisibility (Variables|Default|Getleftpage1) false false)
  (Variables|Default|SetpageFlippedRight? true)
  (Utilities|FlowControl|Delay 0.3)
  (Variables|Default|SetpageFlippedRight? false)
  (Utilities|FlowControl|Delay 0.5)
  (Rendering|SetVisibility (Variables|Default|Getleftpage2) true false))

(event Custom|close%20book
  (Variables|Default|SetisClosed? true)
  (Rendering|SetVisibility (Variables|Default|Getleftpage2) false false)
  (Utilities|FlowControl|Delay 0.8)
  (Rendering|SetVisibility (Variables|Default|Getcover) true false))

(event Custom|flip%20left
  (Variables|Default|SetpageFlippedLeft? true)
  (Utilities|FlowControl|Delay 0.3)
  (Variables|Default|SetpageFlippedLeft? false))

(event EventBeginPlay
  (Variables|Default|SetisClosed? true)
  (Rendering|SetVisibility (Variables|Default|Getleftpage2) false false)
  (Input|EnableInput (Game|GetPlayerController 0)))

(event Collision|EventActorBeginOverlap
  (params (OtherActor :type Actor%20Object%20Reference)))

(event EventTick
  (params (DeltaSeconds :type Float%20%28single-precision%29)))

(event Input|GamepadEvents|GamepadDPadLeft
  (params (Key :type Key%20Structure :default "AnyKey"))
  (:Pressed
    (CallFunction|FlipLeft)))

(event Input|GamepadEvents|GamepadDPadRight
  (params (Key :type Key%20Structure :default "AnyKey"))
  (:Pressed
    (if (Variables|Default|Getisclosed?)
      (CallFunction|OpenBook)
      (else
        (CallFunction|FlipRight)
        (Variables|Default|Setpagenumber (+ (Variables|Default|Getpagenumber) 1))))))

(event Input|GamepadEvents|GamepadDPadUp
  (params (Key :type Key%20Structure :default "AnyKey"))
  (:Pressed
    (if (Variables|Default|Getisclosed?)
      (CallFunction|OpenBook)
      (else
        (CallFunction|FlipRight)
        (Variables|Default|Setpagenumber (+ (Variables|Default|Getpagenumber) 1))))))

(event Input|GamepadEvents|GamepadDPadDown
  (params (Key :type Key%20Structure :default "AnyKey"))
  (:Pressed
    (CallFunction|FlipLeft)))

(fn ConstructionScript)