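; Closed book actor in the viberoom that pulls out from its place for display when selected and returns when deselected.
; Timelines lerp it between its saved transform and a shelf mid location, rolling or turning it 90 degrees on the way.
; AddToTable and Deselect components are shown with collision and tick only while displayed.
; The add-to-table event currently only prints a message.
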(event Custom|book%20deselcted
  (bind _addtotable (Variables|Default|GetaddToTable))
  (bind _defaultsceneroot (Variables|Default|GetDefaultSceneRoot))
  (bind _newtrack_0 (Timeline|Timeline_1 PlayFromStart)
    (:Update
      (Transformation|SetWorldLocation _defaultsceneroot (Math|Vector|Lerp(Vector) (Variables|Default|Getbookshelfmidlocation) (Variables|Default|Getinitialbooklocation) _newtrack_0) false false)
      (Transformation|SetWorldRotation _defaultsceneroot (Math|Rotator|Lerp(Rotator) (Variables|Default|Getbookfinalrotation) (Variables|Default|Getinitialbookrotation) _newtrack_0) false false))
    (:Finished
      (Variables|Default|SetisDisplaying? false)
      (Development|SetHiddeninGame _addtotable true false)
      (Collision|SetCollisionEnabled _addtotable "NoCollision")
      (Components|Tick|SetComponentTickEnabled _addtotable false))))

(event Custom|book%20added%20to%20table
  (Development|PrintString "book added to table"))

(event Collision|EventActorBeginOverlap
  (params (OtherActor :type Actor%20Object%20Reference)))

(event EventTick
  (params (DeltaSeconds :type Float%20%28single-precision%29)))

(event EventBookSelected
  (bind _defaultsceneroot (Variables|Default|GetDefaultSceneRoot))
  (bind _addtotable (Variables|Default|GetaddToTable))
  (if (not (Variables|Default|GetisDisplaying?))
    (Variables|Default|Setinitialbooklocation (Transformation|GetWorldLocation _defaultsceneroot))
    (bind _output_get (Variables|Default|Setinitialbookrotation (Transformation|GetWorldRotation _defaultsceneroot)))
    (Variables|Default|Setbookfinalrotation (Math|Rotator|CombineRotators _output_get "0,90.000000, 0"))
    (bind _newtrack_0 (Timeline|Timeline_0 PlayFromStart)
      (:Update
        (Transformation|SetWorldLocation _defaultsceneroot (Math|Vector|Lerp(Vector) (Variables|Default|Getinitialbooklocation) (Variables|Default|Getbookshelfmidlocation) _newtrack_0) false false)
        (Transformation|SetWorldRotation _defaultsceneroot (Math|Rotator|Lerp(Rotator) (Variables|Default|Getinitialbookrotation) (Variables|Default|Getbookfinalrotation) _newtrack_0) false false))
      (:Finished
        (Development|SetHiddeninGame _addtotable false false)
        (Collision|SetCollisionEnabled _addtotable "QueryAndPhysics")
        (Components|Tick|SetComponentTickEnabled _addtotable true)
        (Variables|Default|SetisDisplaying? true)))))

(event EventBeginPlay
  (bind _addtotable (Variables|Default|GetaddToTable))
  (Development|SetHiddeninGame _addtotable true false)
  (Collision|SetCollisionEnabled _addtotable "NoCollision")
  (Components|Tick|SetComponentTickEnabled _addtotable false))

(fn ConstructionScript)